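; Player character for a plane-constrained platformer, with movement, jumping, dash, run, ledge-style climb launch and interaction.
; Move adds a slight off-axis nudge to control facing; landing and falling events maintain double-jump and coyote-time state.
; Debug keys drive a timer-gated dash and a speed multiplier applied on Tick, while climbing uses a line trace.
; Interaction uses a sphere trace with BPI_Interaction or BPPlayerInteraction, and soft platforms toggle capsule collision.
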(event Custom|CustomEvent
  ;[0 0 0 0.5] Climb
  (Variables|Default|SetCanClimb true))

(event Custom|On%20Landed
  (params (Hit :type Hit%20Result%20Structure%20%28by%20ref%29))
  ;[0.15 0.15 0.15 0.502] On Landed - Reset the double jump flag
  (Variables|SideScrolling|SetHas%20Double%20Jumped false))

(event Custom|On%20Movement%20Mode%20Changed
  (params (Character :type Character%20Object%20Reference) (PrevMovementMode :type EMovementMode%20Enum :default "MOVE_None") (PreviousCustomMode :type Byte))
  ;[0.15 0.15 0.15 0.5] Movement Mode Changes
  ;;[0.15 0.15 0.15 0.5] Have we just started falling?
  (if (Utilities|Enum|Equal(Enum) (Variables|/Script/Engine.CharacterMovementComponent|GetMovementMode (Variables|/Script/Engine.Character|GetCharacterMovement Character)) "MOVE_Falling")
    ;;[0.15 0.15 0.15 0.5] Save the game time when we started falling so we can keep track of Coyote Time jumps
    (Variables|CoyoteTime|SetLast%20Falling%20Time (Utilities|Time|GetTimeSeconds))))

(event Custom|Tick_Climb
  (bind (_start _end) (|TraceVector))
  ;[0 0 0 0.5] Climb
  (if (and (Variables|Default|GetCanClimb) (AI|Components|NavMovement|IsFalling (Variables|Character|GetCharacterMovement)))
    (bind (_outhit _returnvalue) (Collision|LineTraceForObjects _start _end (Utilities|Array|MakeArray "ObjectTypeQuery1" "ObjectTypeQuery2" "ObjectTypeQuery4") false 0 "ForOneFrame" true "(R=1.000000,G=0.000000,B=0.000000,A=1.000000)" "(R=0.000000,G=1.000000,B=0.000000,A=1.000000)" 0.0))
    (if _returnvalue
      (if (>= (Math|Vector|Distance(Vector) (.Location (Collision|BreakHitResult _outhit)) (.TraceStart (Collision|BreakHitResult _outhit))) 1e+01)
        (Character|LaunchCharacter (Math|Vector|MakeVector 0.0 0.0 (Variables|Default|GetClimbLaunchPower)) false true)
        (Variables|Default|SetCanClimb false)
        (Utilities|Time|SetTimerbyEvent (delegate Custom|CustomEvent) 0.2)))))

(event Custom|ResetDash
  ;[0 0 0 0.5] Dash
  (Variables|Dash|SetCanDash true))

(event Input|EnhancedActionEvents|EnhancedInputActionIA_Interact
  (params (ActionValue :type Boolean) (ElapsedSeconds :type Float%20%28double-precision%29) (TriggeredSeconds :type Float%20%28double-precision%29) (InputAction :type Input%20Action%20Object%20Reference :default "/Game/Variant_SideScroller/Input/Actions/IA_Interact.IA_Interact"))
  (bind _returnvalue (Transformation|GetActorLocation))
  ;[0.15 0.15 0.15 0.502] On Interact Action, Sphere Trace around the Player and send an "Interaction" call via our BPI_Interaction interface. If the actor also has that interface (added via Class Settings) they will receive the call and can activate an "Interaction" event. See BP_SImpleNPC
  (bind _outhit (Collision|SphereTraceForObjects _returnvalue (+ (Math|Vector|MakeVector 1e+02 0.0 0.0) _returnvalue) (Variables|SideScrolling|GetInteraction%20Radius) (Utilities|Array|MakeArray "ObjectTypeQuery3" "ObjectTypeQuery2") false 0 "None"))
  (Class|BPISideScrolling|Interaction(Message) (.HitActor (Collision|BreakHitResult _outhit)) self))

(event Input|EnhancedActionEvents|EnhancedInputActionIA_Jump
  (params (ActionValue :type Boolean) (ElapsedSeconds :type Float%20%28double-precision%29) (TriggeredSeconds :type Float%20%28double-precision%29) (InputAction :type Input%20Action%20Object%20Reference :default "/Game/Input/Actions/IA_Jump.IA_Jump"))
  (Character|Jump))

(event Input|EnhancedActionEvents|EnhancedInputActionIA_Move
  (params (ActionValue :type Vector%202D%20Structure) (ElapsedSeconds :type Float%20%28double-precision%29) (TriggeredSeconds :type Float%20%28double-precision%29) (InputAction :type Input%20Action%20Object%20Reference :default "/Game/Input/Actions/IA_Move.IA_Move"))
  ;[0.15 0.15 0.15 0.5] Move Player
  (CallFunction|Move (.y ActionValue)))

(event EventBeginPlay
  ;[0.15 0.15 0.15 0.5] Initialization - Register event handlers
  (EventDispatchers|BindEventtoLandedDelegate (EventDispatchers|CreateEvent :!event Custom|On%20Landed))
  (EventDispatchers|BindEventtoMovementModeChangedDelegate (EventDispatchers|CreateEvent :!event Custom|On%20Movement%20Mode%20Changed))
  (Variables|Movement|SetBaseWalkSpeed (Variables|/Script/Engine.CharacterMovementComponent|GetMaxWalkSpeed (Variables|Character|GetCharacterMovement)))
  (Actor|Tick|SetActorTickEnabled true))

(event EventTick
  (params (DeltaSeconds :type Float%20%28single-precision%29))
  (|CallParentFunction DeltaSeconds)
  (CallFunction|UpdateWalkSpeed)
  (CallFunction|TickClimb))

(event EventTouchInteractStart
  (bind _returnvalue (Transformation|GetActorLocation))
  ;[0.15 0.15 0.15 0.502] On Interact Action, Sphere Trace around the Player and send an "Interaction" call via our BPI_Interaction interface. If the actor also has that interface (added via Class Settings) they will receive the call and can activate an "Interaction" event. See BP_SImpleNPC
  (bind _outhit (Collision|SphereTraceForObjects _returnvalue (+ (Math|Vector|MakeVector 1e+02 0.0 0.0) _returnvalue) (Variables|SideScrolling|GetInteraction%20Radius) (Utilities|Array|MakeArray "ObjectTypeQuery3" "ObjectTypeQuery2") false 0 "None"))
  (Class|BPISideScrolling|Interaction(Message) (.HitActor (Collision|BreakHitResult _outhit)) self))

(event EventPrimaryThumbstick
  (params (Axis :type Vector%202D%20Structure))
  ;[0.15 0.15 0.15 0.5] Move Player
  (CallFunction|Move (.y Axis)))

(event EventSetSoftCollision
  (params (Enabled :type Boolean))
  ;[0.15 0.15 0.15 0.5] Enable or disable collision response so we can go through soft collision platforms.
  (Collision|SetCollisionResponsetoChannel (Variables|Collision|GetCapsuleComponent) "ECC_GameTraceChannel1" (select Enabled "ECR_Ignore" "ECR_Block")))

(event Input|KeyboardEvents|DebugKeyZ
  (params (Key :type Key%20Structure :default "None") (ActionValue :type Input%20Action%20Value%20Structure))
  ;[0 0 0 0.5] Dash
  (:Pressed
    (if (Variables|Dash|GetCanDash)
      (Character|LaunchCharacter (+ (* (Transformation|GetActorForwardVector) (Variables|Dash|GetDashPower)) "0.000000,0.000000,100.000000") true true)
      (Variables|Dash|SetCanDash false)
      (Utilities|Time|SetTimerbyEvent (delegate Custom|ResetDash) 4.0)
      (Utilities|FlowControl|Delay 0.3)
      (Variables|/Script/Engine.MovementComponent|SetVelocity (Variables|Character|GetCharacterMovement) "0, 0, 0"))))

(event Input|KeyboardEvents|DebugKeyE
  (params (Key :type Key%20Structure :default "None") (ActionValue :type Input%20Action%20Value%20Structure))
  (:Pressed
    (Default|TrytoInteract (Variables|Default|GetBP_PlayerInteraction))))

(event Input|KeyboardEvents|DebugKeyQ
  (params (Key :type Key%20Structure :default "None") (ActionValue :type Input%20Action%20Value%20Structure))
  ;[0 0 0 0.5] Run
  (:Pressed
    (Variables|Movement|Run|SetRunMuliplier 1e+03))
  (:Released
    (Variables|Movement|Run|SetRunMuliplier 1.0)))

(fn ConstructionScript)

(fn CheckforSoftCollision
  (bind _returnvalue (Transformation|GetActorLocation))
  (bind (_outhit _returnvalue_2) (Collision|LineTraceForObjects _returnvalue (- _returnvalue "0.000000,0.000000,1000.000000") (Utilities|Array|MakeArray "ObjectTypeQuery7") false 0 "None"))
  (if _returnvalue_2
    (CallFunction|SetSoftCollision true)))

(fn Move
  (params (Y%20Axis :type Float%20%28double-precision%29))
  ;[0.15 0.15 0.15 0.502] Movement Input - Gamepad By forcing a slight movement in Y we can ensure that the player always faces and rotates towards the camera. This Y movement is cancelled out by the plane constraint on the character movement controller.
  (if (not (Variables|SideScrolling|GetHas%20Wall%20Jumped))
    (Pawn|Input|AddMovementInput (Math|Vector|SelectVector "1.000000,0.100000,0.000000" "1.000000,-0.100000,0.000000" (> Y%20Axis 0.0)) Y%20Axis false)
    (Variables|SideScrolling|SetAction%20Value%20Y Y%20Axis)))

(fn UpdateWalkSpeed
  (Variables|/Script/Engine.CharacterMovementComponent|SetMaxWalkSpeed (Variables|Character|GetCharacterMovement) (* (Variables|Movement|GetBaseWalkSpeed) (Variables|Movement|Run|GetRunMuliplier))))

(fn GetHasDoubleJump
  (return (Variables|SideScrolling|GetHas%20Double%20Jumped)))

(fn GetHasWallJumped
  (return (Variables|SideScrolling|GetHas%20Wall%20Jumped)))
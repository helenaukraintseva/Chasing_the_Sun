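; BP_LaunchPad is a launch pad actor that pushes overlapping Characters with a continuous force.
; Each Tick it adds force to their CharacterMovement, scaled by LaunchPower and world delta time.
; GetLaunchDirection returns the normalized vector from the pad to player 0, so every overlapping Character shares that direction.
; A one-shot LaunchCharacter branch for the player is disconnected, and the begin-overlap event is empty.
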(event `self.ReceiveActorBeginOverlap`
  (params (OtherActor :type "Actor Object Reference")))

(event `self.ReceiveTick`
  (params (DeltaSeconds :type "Float (single-precision)"))
  (for _array_element (`self.GetOverlappingActors` "/Script/Engine.Character")
    (`CharacterMovementComponent.AddForce` (`Character.CharacterMovement` _array_element) (* (`self.GetLaunchDirection`) (`self.LaunchPower`) (`GameplayStatics.GetWorldDeltaSeconds`)))))

(fn `GetLaunchDirection`
  (returns (ReturnValue :type "Vector Structure"))
  (return (`KismetMathLibrary.Normal` (- (`self.K2_GetActorLocation` (`GameplayStatics.GetPlayerCharacter` 0)) (`self.K2_GetActorLocation`)))))

(fn `UserConstructionScript`)